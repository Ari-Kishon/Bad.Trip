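; TimerBlock is a platform block that alternates between large and quarter-size on a repeating five-second timer.
; BeginPlay starts the looping timer on ChangeSize, which plays the BlockTimer sound, scales the actor by a factor of four and flips IsLarge.
; ChangeState would set visibility with the same sound but is not called here, and the construction script's initial visibility and size logic is disconnected.
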(event EventBeginPlay
  (Utilities|Time|SetTimerbyFunctionName 0 "ChangeSize" 5.0 true))

(fn ConstructionScript)

(fn ChangeState
  (Rendering|SetActorHiddenInGame (not (Variables|Rendering|GetbHidden)))
  (Audio|PlaySoundatLocation "/Game/BadTripAssests/SFX/BlockTimer.BlockTimer" (Transformation|GetActorLocation) "0, 0, 0" 0.3 1.0 0.0 0 0 0))

(fn ChangeSize
  (bind _returnvalue (Class|Actor|GetActorRelativeScale3D))
  (Audio|PlaySoundatLocation "/Game/BadTripAssests/SFX/BlockTimer.BlockTimer" (Transformation|GetActorLocation) "0, 0, 0" 0.2 1.0 0.0 0 0 0)
  (if (Variables|Default|Getis_large)
    (Transformation|SetActorRelativeScale3D (/ _returnvalue 4))
    (Variables|Default|Setis_large (not (Variables|Default|Getis_large)))
    (else
      (Transformation|SetActorRelativeScale3D (* _returnvalue 4))
      (Variables|Default|Setis_large (not (Variables|Default|Getis_large))))))