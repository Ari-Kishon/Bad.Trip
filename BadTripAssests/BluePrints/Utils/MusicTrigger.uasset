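; MusicTrigger is an overlap-driven actor that plays a chosen song while something is inside it.
; On overlap begin it spawns the SongToPlay sound at the actor's location at a lowered pitch and stores the component in Song.
; On overlap end it stops that sound, without filtering which actor overlapped.
; Unconnected construction logic would label a text render with the song name.
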(event EventBeginPlay)

(event Collision|EventActorBeginOverlap
  (params (OtherActor :type Actor%20Object%20Reference))
  (bind _returnvalue (Audio|SpawnSoundatLocation (Variables|Default|Getsong_to_play) (Transformation|GetActorLocation) "0, 0, 0" 1.0 0.7 0.0 0 0))
  (Variables|Default|SetSong _returnvalue))

(event Collision|EventActorEndOverlap
  (params (OtherActor :type Actor%20Object%20Reference))
  (Audio|Components|Audio|Stop (Variables|Default|GetSong)))

(fn ConstructionScript)