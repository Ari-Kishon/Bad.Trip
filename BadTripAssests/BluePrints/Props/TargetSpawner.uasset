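; Target spawner actor that keeps adding test targets to the level around its own position.
; On BeginPlay a looping timer calls SpawnTarget every two seconds, with no cap on how many accumulate.
; Each call spawns a Target_Test with a set starting health at a random integer offset from the spawner, always on the positive X and Y side and raised above it.
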(event Collision|EventActorBeginOverlap
  (params (OtherActor :type Actor%20Object%20Reference)))

(event EventBeginPlay
  (Utilities|Time|SetTimerbyFunctionName 0 "SpawnTarget" 2.0 true))

(fn ConstructionScript)

(fn SpawnTarget
  (Game|SpawnActorfromClass "/Game/Target_Test.Target_Test_C" (Math|Transform|MakeTransform (+ (Transformation|GetActorLocation) (Math|Vector|MakeVector (Math|Conversions|ToFloat(Integer) (Math|Random|RandomIntegerinRange 50 700)) (Math|Conversions|ToFloat(Integer) (Math|Random|RandomIntegerinRange 50 700)) (Math|Conversions|ToFloat(Integer) (Math|Random|RandomIntegerinRange 400 700))))) "Undefined" 0 3 0))